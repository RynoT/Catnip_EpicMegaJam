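; BP_CatCharacter is the player cat's Blueprint, handling HUD creation and the pause menu.
; Possession by a PlayerController adds UI_HUD; pressing Pause freezes the game and shows UI_PauseMenu with the cursor.
; A Gate swallows that press's release, so a later release or the Unpause event resumes play.
; Resuming removes the menu and hides the cursor, but is blocked when DefaultGameMode's LifeCount is not above zero.
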(event Custom|Event%20Unpause
  (Utilities|FlowControl|Sequence
    (:then_0
      (Utilities|FlowControl|Gate false :!label _label
        (:Exit
          (if (Game|IsGamePaused)
            (bind _asdefault_game_mode (Utilities|Casting|CastToDefaultGameMode (Game|GetGameMode))
              (:then
                (if (> (Variables|/Script/Catnip.DefaultGameMode|GetLifeCount _asdefault_game_mode) 0)
                  (Game|SetGamePaused false :!label _label_2)
                  (Widget|RemovefromParent (Variables|Default|GetPause%20UI))
                  (Variables|/Script/Engine.PlayerController|SetbShowMouseCursor (Game|GetPlayerController 0) false)))
              (:CastFailed
                (goto _label_2)))))))
    (:then_1
      (goto _label Open))))

(event EventPossessed
  (params (NewController :type Controller%20Object%20Reference))
  (Utilities|Casting|CastToPlayerController NewController)
  (bind _returnvalue (UserInterface|CreateWidget "/Game/UI/UI_HUD.UI_HUD_C"))
  (bind _output_get (Variables|Default|SetHUD%20UI _returnvalue))
  (UserInterface|Viewport|AddtoViewport _output_get 0))

(event Input|ActionEvents|InputActionPause
  (params (Key :type Key%20Structure :default "None"))
  (:Pressed
    (if (not (Game|IsGamePaused))
      (Game|SetGamePaused true)
      (bind _returnvalue (UserInterface|CreateWidget "/Game/UI/UI_PauseMenu.UI_PauseMenu_C"))
      (bind _output_get (Variables|Default|SetPause%20UI _returnvalue))
      (UserInterface|Viewport|AddtoViewport _output_get 0)
      (Variables|/Script/Engine.PlayerController|SetbShowMouseCursor (Game|GetPlayerController 0) true)
      (goto _label Close)))
  (:Released
    (Utilities|FlowControl|Sequence
      (:then_0
        (Utilities|FlowControl|Gate false :!label _label
          (:Exit
            (if (Game|IsGamePaused)
              (bind _asdefault_game_mode (Utilities|Casting|CastToDefaultGameMode (Game|GetGameMode))
                (:then
                  (if (> (Variables|/Script/Catnip.DefaultGameMode|GetLifeCount _asdefault_game_mode) 0)
                    (Game|SetGamePaused false :!label _label_2)
                    (Widget|RemovefromParent (Variables|Default|GetPause%20UI))
                    (Variables|/Script/Engine.PlayerController|SetbShowMouseCursor (Game|GetPlayerController 0) false)))
                (:CastFailed
                  (goto _label_2)))))))
      (:then_1
        (goto _label Open)))))

(fn ConstructionScript)