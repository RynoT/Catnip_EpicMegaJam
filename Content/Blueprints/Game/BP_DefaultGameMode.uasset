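; Default game mode Blueprint that handles the game's fail and completion outcomes.
; On failure it pauses the game and shows a failed-menu widget.
; On completion it triggers a fade on the cat character's HUD and opens the HouseMap level once that fade completes.
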(event Custom|Event%20FadeComplete
  (Game|OpenLevel(byName) "HouseMap"))

(event EventOnGameCompleted
  (bind _asbp_cat_character (Utilities|Casting|CastToBP_CatCharacter (Game|GetPlayerCharacter 0)))
  (EventDispatchers|BindEventtoOnFadeComplete (Variables|/Game/Blueprints/Player/BP_CatCharacter.BP_CatCharacter_C|GetHUD%20UI _asbp_cat_character) (delegate Custom|Event%20FadeComplete))
  (Default|EventTriggerFade (Variables|/Game/Blueprints/Player/BP_CatCharacter.BP_CatCharacter_C|GetHUD%20UI _asbp_cat_character)))

(event EventOnGameFailed
  (Game|SetGamePaused true)
  (bind _returnvalue (UserInterface|CreateWidget "/Game/UI/UI_FailedMenu.UI_FailedMenu_C"))
  (UserInterface|Viewport|AddtoViewport _returnvalue 0))

(fn ConstructionScript)