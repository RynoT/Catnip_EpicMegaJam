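; BP_RingHandler sets up a beat-ring run and relays each ring's success or failure to the audio actor.
; On BeginPlay it configures spawn rules from a hardcoded beat list, covering ring and obstacle meshes, decorative animal meshes, offset and rotation.
; Success and fail events drive effects and accents on CompletedDoriansRunActor, which is flagged dead once failures reach a cumulative limit.
; Radius rules are present but never run.
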(event Custom|Event%20On%20Success
  (params (RingIndex :type Integer))
  (bind _audiobp (Variables|Default|GetAudioBP))
  (Development|PrintString "Ring Success")
  (Default|PianoEffect _audiobp)
  (Variables|/Game/Master_Audio/2_CompletedCue/CompletedDoriansRunActor.CompletedDoriansRunActor_C|SetRingSuccess _audiobp true)
  (Default|PlayAccent (Variables|Default|GetAudioBP)))

(event Custom|Event%20On%20Fail
  (params (RingIndex :type Integer))
  (Development|PrintString "Ring Fail")
  (Math|Integer|IncrementInt (Variables|Default|GetFailCount)
    (:%20%20
      (Variables|/Game/Master_Audio/2_CompletedCue/CompletedDoriansRunActor.CompletedDoriansRunActor_C|SetRingSuccess (Variables|Default|GetAudioBP) false)
      (if (>= (Variables|Default|GetFailCount) 9)
        (Variables|/Game/Master_Audio/2_CompletedCue/CompletedDoriansRunActor.CompletedDoriansRunActor_C|SetisDead (Variables|Default|GetAudioBP) true))
      (Default|PlayAccent (Variables|Default|GetAudioBP)))))

(event EventBeginPlay
  (bind (_x _y _z) (Math|Vector|BreakVector "0.901042,0.637516,0.049874"))
  (|CallParentFunction)
  (Utilities|FlowControl|Sequence
    (:then_0
      (EventDispatchers|BindEventtoOnBeatRingSuccess (delegate Custom|Event%20On%20Success))
      (EventDispatchers|BindEventtoOnBeatRingFail (delegate Custom|Event%20On%20Fail))
      (bind _outactors (Actor|GetAllActorsOfClass "/Game/Master_Audio/2_CompletedCue/CompletedDoriansRunActor.CompletedDoriansRunActor_C"))
      (Variables|Default|SetAudioBP (Utilities|Array|Get(acopy) _outactors)))
    (:then_1
      (Class|RingHandler|SpawnRuleSetBeatRings (Utilities|String|JoinStringArray (Utilities|Array|MakeArray "32" "40" "64" "72" "80" "96" "112" "128" "144" "162" "166" "170" "174" "192" "216" "224" "236" "256" "278" "282" "286" "290" "296" "304" "320" "324" "326" "328" "332" "334" "342" "352" "356" "360" "362" "368" "372" "376" "378" "400" "402" "404" "406" "408" "410" "412" "414" "416" "424" "432" "446" "448" "452" "456" "460" "462" "464" "468" "472" "476" "478" "480" "488" "496" "562" "566" "570" "574" "576" "578" "582" "114" "454" "458" "460" "461" "462" "464" "466" "467" "468" "470" "480" "482" "485" "486" "488" "490" "493" "494" "511" "512" "514" "515" "516" "519" "520" "522" "523" "524" "527" "528" "530" "531" "532" "535" "536" "538" "539" "540" "543" "544") ", ") (Utilities|Array|MakeArray "/Game/Meshes/ring_1.ring_1" "/Game/Meshes/ring_2.ring_2") "/Game/Material/RingObjectsPink.RingObjectsPink" (Math|Color|MakeColor (Math|Conversions|ToByte(Integer) (Math|Float|Truncate (* 255 _z))) (Math|Conversions|ToByte(Integer) (Math|Float|Truncate (* 255 _y))) (Math|Conversions|ToByte(Integer) (Math|Float|Truncate (* 255 _x))) 255) (Utilities|Array|MakeArray "/Game/Meshes/Barrier_1.Barrier_1" "/Game/Meshes/Barrier_2.Barrier_2" "/Game/Meshes/Barrier_3.Barrier_3" "/Game/Meshes/Barrier_4.Barrier_4" "/Game/Meshes/Barrier_5.Barrier_5") "/Game/Material/CollisionRing_Material_Inst.CollisionRing_Material_Inst")
      (Class|RingHandler|SpawnRuleSetMesh 12 "/Game/Meshes/fish_high.fish_high" "/Game/Material/RingObjectsMaterial_Inst.RingObjectsMaterial_Inst" "MultipleMesh" false)
      (Class|RingHandler|SpawnRuleSetMesh 7 "/Game/Meshes/Dog_high.Dog_high" "/Game/Material/RingObjectsMaterial_Inst.RingObjectsMaterial_Inst" "SingleMesh" false)
      (Class|RingHandler|SpawnRuleSetOffset 3 1.0 "Incremental")
      (Class|RingHandler|SpawnRuleSetRotation 5 1e+01 1e+01 -1.0)
      (Variables|Default|SetFailCount 0)
      (Variables|/Game/Master_Audio/2_CompletedCue/CompletedDoriansRunActor.CompletedDoriansRunActor_C|SetisDead (Variables|Default|GetAudioBP) false))))

(fn ConstructionScript)