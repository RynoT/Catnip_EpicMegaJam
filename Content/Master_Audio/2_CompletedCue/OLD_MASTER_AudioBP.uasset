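; Music director Blueprint that plays the level's track through TimeSynth and syncs visual effects to it.
; Quantized bar and quarter-note events update playback state and a beat counter, whose hard-coded cues fire timelines for pulses, colour transitions and opacity fades.
; Those timelines and the envelope follower's amplitude write to material parameter collections.
; Accent events play success or pain stingers, while death queues the ending clip and fades out the main loop.
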(event Custom|StartMusic
  ;[1 1 1] Check if Music is already Playing
  (if (not (Variables|Default|GetbMusicPlaying))
    (Variables|Default|SetbMusicPlaying true)
    (|InitState)
    ;[1 1 1] Set up Quantization Delegates
    (Class|TimeSynthComponent|AddQuantizationEventDelegate (Variables|Default|GetTimeSynth) "Bar" (EventDispatchers|CreateEvent :!event Custom|OnBarEvent))
    (Class|TimeSynthComponent|AddQuantizationEventDelegate (Variables|Default|GetTimeSynth) "QuarterNote" (EventDispatchers|CreateEvent :!event Custom|OnBeatEvent))
    (Utilities|FlowControl|Sequence
      (:then_0
        ;[1 1 1] Set initial values for Volume Groups
        (CallFunction|SetVolumeGroups))
      (:then_1
        ;[1 1 1] (Re)trigger Main Loop
        (Utilities|FlowControl|Sequence
          (:then_0
            (bind _returnvalue (Class|TimeSynthComponent|PlayClip (Variables|Default|GetTimeSynth) "/Game/Master_Audio/MainMusic.MainMusic" "/Game/Master_Audio/VolumeGroups/DoriansRun_Hi.DoriansRun_Hi"))
            (Variables|Default|SetMainLoopHigh _returnvalue))
          (:then_2
            (Variables|Default|SetbMainLoopQueued true)
            (Variables|Default|SetbMainLoopStarted true)))))))

(event Custom|LevelFinished
  ;[0.1183 0.2471 1] BEATS
  ;;[1 0.05157 0.08141] END
  ;;;[1 1 1] If Ending Clip is done, Update State
  (Variables|Default|SetbEndingClipStarted false)
  (Variables|Default|SetbMusicPlaying false)
  (Components|Activation|Deactivate (Variables|Default|GetTimeSynth)))

(event Custom|PlayAccent
  ;[1 1 1] STINGERS
  (if (Variables|Default|GetbMusicPlaying)
    (Variables|Default|SetbAccentPlaying true)
    (if (Variables|Default|GetRingSuccess)
      (bind _returnvalue (Class|TimeSynthComponent|PlayClip (Variables|Default|GetTimeSynth) "/Game/Master_Audio/Success.Success" "/Game/Master_Audio/VolumeGroups/DoriansRun_success.DoriansRun_success"))
      (Variables|Default|SetMainLoopsuccess _returnvalue)
      (elif (Variables|Default|GetisDead)
        (CallFunction|EndMusic)
        (Variables|Default|SetisDead false)
        ;[1 0.09236 0.08333] DAMAGE EFFECTS
        ;;[1 1 1] DEATH
        (Rendering|Material|SetScalarParameterValue "/Game/Material/Mat_parameters.Mat_parameters" "None" 0.0 :!class /Script/Engine.KismetMaterialLibrary)
        (else
          (bind _returnvalue_2 (Class|TimeSynthComponent|PlayClip (Variables|Default|GetTimeSynth) "/Game/Master_Audio/Pain.Pain" "/Game/Master_Audio/VolumeGroups/DoriansRun_Lo.DoriansRun_Lo"))
          (Variables|Default|SetMainLoopLow _returnvalue_2)
          ;;[1 1 1] PAIN
          (Rendering|Material|SetScalarParameterValue "/Game/Material/Mat_parameters.Mat_parameters" "None" 0.0 :!class /Script/Engine.KismetMaterialLibrary))))))

(event Custom|OnBeatEvent
  (params (QuantizationType :type ETimeSynthEventQuantization%20Enum :default "None") (NumBars :type Integer) (Beat :type Float%20%28single-precision%29))
  ;[0.1183 0.2471 1] BEATS
  (Variables|Default|SetCurrentBeat Beat)
  (Utilities|FlowControl|Sequence
    (:then_0
      (Utilities|FlowControl|Sequence
        (:then_0
          ;;[1 1 1] Free up Accent Every Beat
          (Variables|Default|SetbAccentPlaying false))
        (:then_3
          ;;[1 0.05157 0.08141] END
          ;;;[1 1 1] If Ending Clip is done, Update State
          (if (>= (Variables|Default|GetEndingClipCount) (Variables|Default|GetEndingClipLength))
            (Variables|Default|SetbEndingClipStarted false)
            (Variables|Default|SetbMusicPlaying false)
            (Components|Activation|Deactivate (Variables|Default|GetTimeSynth))))))
    (:then_1
      (|UpdateBeatCounters))
    (:then_2
      ;;[0.0235 1 0.08355] RING SPAWN
      ;;;[1 1 1] Start Beat after intro
      (if (>= (Variables|Default|GetCurrentBeatCount) 16)
        (CallFunction|BeatEffect)
        ;[0.9468 1 0.9341] Post process effects
        (Utilities|FlowControl|Sequence
          (:then_0
            ;;[0.1317 0.85 1] Transition to/from Turquiose
            (if (== (Variables|Default|GetCurrentBeatCount) 160)
              (bind _transition (Timeline|SkySphereTransition PlayFromStart)
                (:Update
                  (Rendering|Material|SetScalarParameterValue "/Game/Material/Mat_parameters.Mat_parameters" "PostProcessAmount" (* _transition 3.0) :!class /Script/Engine.KismetMaterialLibrary)
                  (Rendering|Material|SetScalarParameterValue "/Game/Material/Mat_parameters.Mat_parameters" "ColourBlend" (- 1.0 _transition) :!class /Script/Engine.KismetMaterialLibrary)))))
          (:then_1
            (if (== (Variables|Default|GetCurrentBeatCount) 190)
              (Timeline|SkySphereTransition ReverseFromEnd)))
          (:then_2
            ;;[1 0.2661 0.9438] Transition to/from pink
            (if (== (Variables|Default|GetCurrentBeatCount) 228)
              (Utilities|FlowControl|Sequence
                (:then_0
                  (bind _transition_2 (Timeline|Timeline_7 PlayFromStart)
                    (:Update
                      (Rendering|Material|SetScalarParameterValue "/Game/Material/Mat_parameters.Mat_parameters" "PostProcessAmount" (* _transition_2 3.0) :!class /Script/Engine.KismetMaterialLibrary)
                      (Rendering|Material|SetScalarParameterValue "/Game/Material/Mat_parameters.Mat_parameters" "ColourBlend" _transition_2 :!class /Script/Engine.KismetMaterialLibrary)))))))
          (:then_3
            (if (== (Variables|Default|GetCurrentBeatCount) 276)
              (Variables|Default|Setintensesection false)
              (Timeline|Timeline_7 ReverseFromEnd)))
          (:then_4)
          (:then_5))))
    (:then_3
      ;;;[1 1 1] Play piano on cue
      (for _array_element (Variables|Default|GetPiano_Cues)
        (if (== (Variables|Default|GetCurrentBeatCount) _array_element)
          (CallFunction|PianoEffect))))
    (:then_4
      ;;;[1 1 1] Expanse Effect
      (for _array_element_2 (Variables|Default|GetExpanse_Cues)
        (if (== (Variables|Default|GetCurrentBeatCount) _array_element_2)
          (CallFunction|ExpanseEffect))))
    (:then_5
      (if (== (Variables|Default|GetCurrentBeatCount) 118)
        (Utilities|FlowControl|Sequence
          (:then_0
            (bind _newtrack_0 (Timeline|Timeline_8 PlayFromStart)
              (:Update
                (Rendering|Material|SetScalarParameterValue "/Game/Material/Mat_parameters.Mat_parameters" "RingOpacity_Scalar" _newtrack_0 :!class /Script/Engine.KismetMaterialLibrary))))
          (:then_1
            (bind _newtrack_0_2 (Timeline|Timeline_10 PlayFromStart)
              (:Update
                (Rendering|Material|SetScalarParameterValue "/Game/Material/Beat_Param.Beat_Param" "GodCat_Opacity" _newtrack_0_2 :!class /Script/Engine.KismetMaterialLibrary)))))
        (elif (== (Variables|Default|GetCurrentBeatCount) 300)
          (Utilities|FlowControl|Sequence
            (:then_0
              (bind _newtrack_0_3 (Timeline|Timeline_9 PlayFromStart)
                (:Update
                  (Rendering|Material|SetScalarParameterValue "/Game/Material/Mat_parameters.Mat_parameters" "RingOpacity_Scalar" _newtrack_0_3 :!class /Script/Engine.KismetMaterialLibrary))))
            (:then_1
              (Timeline|Timeline_10 PlayFromStart))))))))

(event Custom|OnBarEvent
  (params (QuantizationType :type ETimeSynthEventQuantization%20Enum :default "None") (NumBars :type Integer) (Beat :type Float%20%28single-precision%29))
  (if (Variables|Default|GetbMusicPlaying)
    (Variables|Default|SetCurrentBar NumBars)
    (Utilities|FlowControl|Sequence
      (:then_0
        (|UpdateStates))
      (:then_1))))

(event Custom|Piano_Effect
  ;[0 0 0] Pulse Effects
  ;;[1 1 1] Piano Effect
  (Utilities|FlowControl|Sequence
    (:then_0
      ;;;[1 1 1] Tunnel Legnth
      (bind _newtrack_0 (Timeline|Timeline_1 PlayFromStart)
        (:Update
          (Rendering|Material|SetScalarParameterValue "/Game/Material/Beat_Param.Beat_Param" "Piano_Beat" _newtrack_0 :!class /Script/Engine.KismetMaterialLibrary))))
    (:then_1
      (bind _newtrack_0_2 (Timeline|Splash PlayFromStart)
        (:Update
          (Rendering|Material|SetScalarParameterValue "/Game/Material/Mat_parameters.Mat_parameters" "Pulse" _newtrack_0_2 :!class /Script/Engine.KismetMaterialLibrary))))
    (:then_2
      (bind _newtrack_0_3 (Timeline|Timeline_3 PlayFromStart)
        (:Update
          (Rendering|Material|SetScalarParameterValue "/Game/Material/Mat_parameters.Mat_parameters" "BarScale" (* 0.0 _newtrack_0_3) :!class /Script/Engine.KismetMaterialLibrary))))))

(event Custom|EndMusic
  ;[1 1 1] Check if Music is actually playing and not already marked for End
  (if (and (Variables|Default|GetbMusicPlaying) (not (Variables|Default|GetbMarkMusicToEnd)))
    (Variables|Default|SetbMarkMusicToEnd true)))

(event Custom|Event%20Start
  (Utilities|FlowControl|Sequence
    (:then_0
      (bind _outactors (Actor|GetAllActorsOfClass "/Game/Blueprints/Level/BP_RingHandler.BP_RingHandler_C"))
      (Variables|Default|SetRingHandler (Utilities|Array|Get(acopy) _outactors))
      (bind _outactors_2 (Actor|GetAllActorsOfClass "/Script/Catnip.CatCharacter"))
      (Variables|Default|SetCat (Utilities|Array|Get(acopy) _outactors_2))
      (Variables|Default|SetPulsing? false)
      (bind _outactors_3 (Actor|GetAllActorsOfClass "/Script/Engine.PostProcessVolume"))
      (Variables|Default|SetPostProcessVolume (Utilities|Array|Get(acopy) _outactors_3))
      (bind _structout (Utilities|Struct|SetmembersinPostProcessSettings (Utilities|Struct|MakePostProcessSettings (Utilities|Struct|MakeWeightedBlendables (Utilities|Array|MakeArray (Utilities|Struct|MakeWeightedBlendable 1.0 "/Game/Material/Skyblack.SkyBlack") (Utilities|Struct|MakeWeightedBlendable 0.0 "/Game/Material/SkyTurquoise.SkyTurquoise") (Utilities|Struct|MakeWeightedBlendable 0.0 "/Game/Material/SkyPink.SkyPink"))))))
      (Variables|/Script/Engine.PostProcessVolume|SetSettings (Variables|Default|GetPostProcessVolume) _structout)
      (Variables|Default|Setintensesection false))
    (:then_2
      ;[1 1 1] MASTER EVENTS
      ;;[0.381 1 0.2488] StartMusic (delayed by 4 beats)
      (CallFunction|StartMusic))))

(event Custom|Beat_Effect
  (bind _currentbeatcount (Variables|Default|GetCurrentBeatCount))
  (bind _returnvalue (>= _currentbeatcount 276))
  ;[0 0 0] Pulse Effects
  ;;[1 1 1] Beat Effect
  (Utilities|FlowControl|Sequence
    (:then_0
      (bind _newtrack_0 (Timeline|Timeline_0 PlayFromStart)
        (:Update
          (Rendering|Material|SetScalarParameterValue "/Game/Material/Mat_parameters.Mat_parameters" "Beat_Scale" (* (Class|TimeSynthComponent|GetEnvelopeFollowerValue (Variables|Default|GetTimeSynth)) _newtrack_0) :!class /Script/Engine.KismetMaterialLibrary))))
    (:then_1
      (if (not (Variables|Default|GetPulsing?))
        (if (== (Math|Integer|%(Integer) _currentbeatcount 2) 0)
          (if (not _returnvalue)
            (bind _newtrack_0_2 (Timeline|Timeline_4 PlayFromStart)
              (:Update
                (Rendering|Material|SetScalarParameterValue "/Game/Material/Mat_parameters.Mat_parameters" "ScalarPerBeat" _newtrack_0_2 :!class /Script/Engine.KismetMaterialLibrary))))
          (elif (>= _currentbeatcount 224)
            (if (not _returnvalue)
              (Timeline|Timeline_4 PlayFromStart))))))))

(event Custom|Expanse%20Effect
  ;[0 0 0] Pulse Effects
  ;;[1 1 1] Expanse Effect
  (bind _newtrack_0 (Timeline|Timeline_5 PlayFromStart)
    (:Update
      (Rendering|Material|SetScalarParameterValue "/Game/Material/Mat_parameters.Mat_parameters" "Scalar" _newtrack_0 :!class /Script/Engine.KismetMaterialLibrary)
      (Rendering|Material|SetScalarParameterValue "/Game/Material/Mat_parameters.Mat_parameters" "Pulse" 1.0 :!class /Script/Engine.KismetMaterialLibrary)
      (Utilities|FlowControl|DoOnce false :!label _label
        (:Completed
          (Variables|Default|SetPulsing? true))))
    (:Finished
      (Variables|Default|SetPulsing? false)
      (goto _label Reset))))

(event EventBeginPlay)

(event EventTick
  (params (DeltaSeconds :type Float%20%28single-precision%29))
  ;[0 1 0.08243] AUDIO AMPLITUDE
  (Rendering|Material|SetScalarParameterValue "/Game/Material/Mat_parameters.Mat_parameters" "GlobalAmplitude" (Class|TimeSynthComponent|GetEnvelopeFollowerValue (Variables|Default|GetTimeSynth)) :!class /Script/Engine.KismetMaterialLibrary)
  (if (Variables|Default|GetbMarkMusicToEnd)
    (Utilities|FlowControl|Sequence
      (:then_0
        ;[1 1 1] If Music Marked to End, but Ending Clips not Queued nor Started, Queue them.
        (if (Math|Boolean|ANDBoolean (not (Variables|Default|GetbEndingClipQueued)) (not (Variables|Default|GetbEndingClipStarted)) (not (Variables|Default|GetbMelodyPlaying)))
          ;[1 1 1] Queue Ending Clips
          (Utilities|FlowControl|Sequence
            (:then_0
              (bind _returnvalue (Class|TimeSynthComponent|PlayClip (Variables|Default|GetTimeSynth) "/Game/Master_Audio/Dead.Dead" "/Game/Master_Audio/VolumeGroups/DoriansRun_Mid.DoriansRun_Mid"))
              (Variables|Default|SetMainLoopMid _returnvalue)
              ;[1 1 1] Queue Main Loop to Stop Playing
              (Class|TimeSynthComponent|StopClipwithFadeOverride (Variables|Default|GetTimeSynth) (Variables|Default|GetMainLoopLow) "QuarterNote" (Utilities|Struct|MakeTimeSynthTimeDef 0 1) :!label _label)
              (Class|TimeSynthComponent|StopClipwithFadeOverride (Variables|Default|GetTimeSynth) (Variables|Default|GetMainLoopHigh) "QuarterNote" (Utilities|Struct|MakeTimeSynthTimeDef 0 1))
              (Variables|Default|SetbMainLoopMarkedForStop true)
              (Variables|Default|SetbMarkMusicToEnd false)
              ;[1 0 0.01929] reset
              (Variables|Default|SetbMusicPlaying false)
              (Utilities|FlowControl|Delay 8.0)
              (Variables|Default|SetCurrentBeatCount -3))
            (:then_2
              (Variables|Default|SetbEndingClipQueued true)))))
      (:then_1
        ;[1 1 1] If Ending Clips have begun and Main Loop is still playing, Queue Main Loop to Stop in one bar
        (if (and (Variables|Default|GetbEndingClipStarted) (Variables|Default|GetbMainLoopPlaying))
          (goto _label))))))

(fn ConstructionScript)

(fn SetHighIntensityVolume
  (params (NormalizedIn :type Float%20%28single-precision%29))
  ;[1 1 1] Non-Linear Mapping of Normalized to non-Normalized dB values.
  (Variables|Default|SetHighIntensityVolumeDB (Math|Float|MapRangeClamped (Math|Trig|Sin(Radians) (* NormalizedIn (Math|Float|MultiplybyPi 0.5))) 0.0 1.0 -6e+01 0.0))
  (CallFunction|SetVolumeGroups))

(fn SetVolumeGroups
  (Class|TimeSynthComponent|SetVolumeGroup (Variables|Default|GetTimeSynth) "/Game/Master_Audio/VolumeGroups/DoriansRun_Lo.DoriansRun_Lo" (Variables|Default|GetLowIntensityVolumeDB) 0.0)
  (Class|TimeSynthComponent|SetVolumeGroup (Variables|Default|GetTimeSynth) "/Game/Master_Audio/VolumeGroups/DoriansRun_Hi.DoriansRun_Hi" (Variables|Default|GetHighIntensityVolumeDB) 0.0)
  (Class|TimeSynthComponent|SetVolumeGroup (Variables|Default|GetTimeSynth) "/Game/Master_Audio/VolumeGroups/DoriansRun_Mid.DoriansRun_Mid" -6.0 0.0)
  (Class|TimeSynthComponent|SetVolumeGroup (Variables|Default|GetTimeSynth) "/Game/Master_Audio/VolumeGroups/DoriansRun_success.DoriansRun_success" -11.0 0.0))